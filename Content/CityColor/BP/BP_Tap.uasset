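; BP_Tap is a tap that toggles running water and a Niagara effect, which starts deactivated on BeginPlay.
; OpenTap alternates through a FlipFlop between two timelines.
; Opening plays Timeline_0 to drive the Water component's Z scale, activating Niagara after a short Delay.
; Closing reverses a separate Timeline_1, collapsing the water's X and Y scale to zero and deactivating Niagara.
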(event EventBeginPlay
  (Components|Activation|Deactivate (Variables|Default|GetNiagara)))

(event EventOpenTap
  (Utilities|FlowControl|FlipFlop
    (:A
      (bind _newtrack_0 (Timeline|Timeline_0 Play)
        (:Update
          (Transformation|SetRelativeScale3D (Variables|Default|GetWater) (Math|Vector|MakeVector 0.5 0.5 _newtrack_0))
          (Utilities|FlowControl|Delay 0.2)
          (Components|Activation|SetActive (Variables|Default|GetNiagara) true false))))
    (:B
      (bind _newtrack_0_2 (Timeline|Timeline_1 Reverse)
        (:Update
          (Transformation|SetRelativeScale3D (Variables|Default|GetWater) (Math|Vector|MakeVector 0.0 0.0 _newtrack_0_2))
          (Components|Activation|SetActive (Variables|Default|GetNiagara) false false))))))

(fn ConstructionScript)
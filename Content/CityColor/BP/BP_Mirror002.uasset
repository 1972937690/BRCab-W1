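; Interactive lit mirror actor with a digital clock, showing a widget while an actor overlaps it.
; Tick splits the system time into six hour, minute and second digit texts; an older manual counting chain never runs.
; While overlapped, custom events toggle light, icon and text glow or switch light color via FlipFlops.
; Brightness events step the emissive strength within clamped limits, blending through timelines on material parameters.
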(event EventBeginPlay
  (Rendering|SetVisibility (Variables|组件|GetWidget) false false))

(event EventOpenMirror
  (bind _staticmesh (Variables|组件|GetStaticMesh))
  (bind _staticmesh_2 (Variables|组件|GetStaticMesh))
  (if (Variables|Default|GetOverlap)
    (Utilities|FlowControl|FlipFlop
      (:A
        (Rendering|Material|SetScalarParameterValueonMaterials _staticmesh_2 "Light Emissive Strength" 0.0)
        (Rendering|Material|SetScalarParameterValueonMaterials _staticmesh "Icon Emissive Strength" 0.0)
        (Rendering|Components|TextRender|SetTextRenderColor (Variables|组件|GetTenSecond) (Math|Color|MakeColor 10 10 10 0))
        (Rendering|Components|TextRender|SetTextRenderColor (Variables|组件|GetOneSecond) (Math|Color|MakeColor 10 10 10 0))
        (Rendering|Components|TextRender|SetTextRenderColor (Variables|组件|GetOneHour) (Math|Color|MakeColor 10 10 10 0))
        (Rendering|Components|TextRender|SetTextRenderColor (Variables|组件|GetTenHour) (Math|Color|MakeColor 10 10 10 0))
        (Rendering|Components|TextRender|SetTextRenderColor (Variables|组件|Get:0) (Math|Color|MakeColor 10 10 10 0))
        (Rendering|Components|TextRender|SetTextRenderColor (Variables|组件|Get:1) (Math|Color|MakeColor 10 10 10 0))
        (Rendering|Components|TextRender|SetTextRenderColor (Variables|组件|GetTenMinute) (Math|Color|MakeColor 10 10 10 0))
        (Rendering|Components|TextRender|SetTextRenderColor (Variables|组件|GetOneMinute) (Math|Color|MakeColor 10 10 10 0)))
      (:B
        (Rendering|Material|SetScalarParameterValueonMaterials _staticmesh_2 "Light Emissive Strength" 1e+01)
        (Rendering|Material|SetScalarParameterValueonMaterials _staticmesh "Icon Emissive Strength" 5.0)
        (Rendering|Components|TextRender|SetTextRenderColor (Variables|组件|GetTenSecond) (Math|Color|MakeColor 255 255 255 0))
        (Rendering|Components|TextRender|SetTextRenderColor (Variables|组件|GetOneSecond) (Math|Color|MakeColor 255 255 255 0))
        (Rendering|Components|TextRender|SetTextRenderColor (Variables|组件|GetOneHour) (Math|Color|MakeColor 255 255 255 0))
        (Rendering|Components|TextRender|SetTextRenderColor (Variables|组件|GetTenHour) (Math|Color|MakeColor 255 255 255 0))
        (Rendering|Components|TextRender|SetTextRenderColor (Variables|组件|Get:0) (Math|Color|MakeColor 255 255 255 0))
        (Rendering|Components|TextRender|SetTextRenderColor (Variables|组件|Get:1) (Math|Color|MakeColor 255 255 255 0))
        (Rendering|Components|TextRender|SetTextRenderColor (Variables|组件|GetTenMinute) (Math|Color|MakeColor 255 255 255 0))
        (Rendering|Components|TextRender|SetTextRenderColor (Variables|组件|GetOneMinute) (Math|Color|MakeColor 255 255 255 0))))))

(event EventTick
  (params (DeltaSeconds :type Float%20%28single-precision%29))
  (bind _returnvalue (Math|DateTime|Now))
  (bind _returnvalue_2 (Class|KismetMathLibrary|GetSecond _returnvalue))
  (bind _returnvalue_3 (Class|KismetMathLibrary|GetMinute _returnvalue))
  (bind _returnvalue_4 (Class|KismetMathLibrary|GetHour _returnvalue))
  (Utilities|FlowControl|Sequence
    (:then_0
      (bind _output_get (Variables|Default|SetOne%20Second (Math|Integer|%(Integer) _returnvalue_2 10)))
      (Rendering|Components|TextRender|SetText (Variables|组件|GetOneSecond) (Utilities|Text|ToText(Integer) _output_get)))
    (:then_1
      (bind _output_get_2 (Variables|Default|SetTen%20Second (/ _returnvalue_2 10)))
      (Rendering|Components|TextRender|SetText (Variables|组件|GetTenSecond) (Utilities|Text|ToText(Integer) _output_get_2)))
    (:then_2
      (bind _output_get_3 (Variables|Default|SetOne%20Minute (Math|Integer|%(Integer) _returnvalue_3 10)))
      (Rendering|Components|TextRender|SetText (Variables|组件|GetOneMinute) (Utilities|Text|ToText(Integer) _output_get_3)))
    (:then_3
      (bind _output_get_4 (Variables|Default|SetTen%20Minute (/ _returnvalue_3 10)))
      (Rendering|Components|TextRender|SetText (Variables|组件|GetTenMinute) (Utilities|Text|ToText(Integer) _output_get_4)))
    (:then_4
      (bind _output_get_5 (Variables|Default|SetOne%20Hour (Math|Integer|%(Integer) _returnvalue_4 10)))
      (Rendering|Components|TextRender|SetText (Variables|组件|GetOneHour) (Utilities|Text|ToText(Integer) _output_get_5)))
    (:then_5
      (bind _output_get_6 (Variables|Default|SetTen%20Hour (/ _returnvalue_4 10)))
      (Rendering|Components|TextRender|SetText (Variables|组件|GetTenHour) (Utilities|Text|ToText(Integer) _output_get_6)))))

(event Collision|EventActorBeginOverlap
  (params (OtherActor :type Actor%20Object%20Reference))
  (Variables|Default|SetOverlap true)
  (Rendering|SetVisibility (Variables|组件|GetWidget) true false))

(event Collision|EventActorEndOverlap
  (params (OtherActor :type Actor%20Object%20Reference))
  (Variables|Default|SetOverlap false)
  (Rendering|SetVisibility (Variables|组件|GetWidget) false false))

(event EventChangeColor
  (bind _staticmesh (Variables|组件|GetStaticMesh))
  (if (Variables|Default|GetOverlap)
    (Utilities|FlowControl|FlipFlop
      (:A
        (Rendering|Material|SetVectorParameterValueonMaterials _staticmesh "LightEmissiveColor" "1.000000,1.000000,1.000000"))
      (:B
        (Rendering|Material|SetVectorParameterValueonMaterials _staticmesh "LightEmissiveColor" "0.650000,0.360000,0.030000")))))

(event EventEnbrightness
  (if (Variables|Default|GetOverlap)
    (Variables|Default|SetTarget%20Light%20Brightness (Math|Float|Clamp(Float) (+ (Variables|Default|GetCurrrent%20Light%20Brightness) 1e+01) 1.0 4e+01))
    (bind _newtrack_0 (Timeline|Timeline_0 PlayFromStart)
      (:Update
        (Rendering|Material|SetScalarParameterValueonMaterials (Variables|组件|GetStaticMesh) "Light Emissive Strength" (Math|Float|Lerp (Variables|Default|GetCurrrent%20Light%20Brightness) (Variables|Default|GetTarget%20Light%20Brightness) _newtrack_0)))
      (:Finished
        (Variables|Default|SetCurrrent%20Light%20Brightness (Variables|Default|GetTarget%20Light%20Brightness))))))

(event EventRebrightness
  (if (Variables|Default|GetOverlap)
    (Variables|Default|SetTarget%20Light%20Brightness (Math|Float|Clamp(Float) (- (Variables|Default|GetCurrrent%20Light%20Brightness) 1e+01) 1.0 4e+01))
    (bind _newtrack_0 (Timeline|Timeline_1 PlayFromStart)
      (:Update
        (Rendering|Material|SetScalarParameterValueonMaterials (Variables|组件|GetStaticMesh) "Light Emissive Strength" (Math|Float|Lerp (Variables|Default|GetCurrrent%20Light%20Brightness) (Variables|Default|GetTarget%20Light%20Brightness) _newtrack_0)))
      (:Finished
        (Variables|Default|SetCurrrent%20Light%20Brightness (Variables|Default|GetTarget%20Light%20Brightness))))))

(fn ConstructionScript)